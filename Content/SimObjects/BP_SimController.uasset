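; Player controller for the spacecraft simulation that owns the HUD and pause menu and relays their actions to BP_SimulationManager.
; It starts with the pause menu open, switching input mode and cursor on each toggle, and feeds manager and route planner logs to the HUD.
; Menu events drive scenario generation, route planning, restart, JSON save/load and parameter edits.
; Scenario generation and restart reposition the pawn to face the spacecraft.
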(event Input|EnhancedActionEvents|EnhancedInputActionIA_Pause
  (params (ActionValue :type Boolean) (ElapsedSeconds :type Float%20%28double-precision%29) (TriggeredSeconds :type Float%20%28double-precision%29) (InputAction :type Input%20Action%20Object%20Reference :default "/Game/Input/InputAction/IA_Pause.IA_Pause"))
  (:Started
    (UI|SwitchPause)))

(event EventBeginPlay
  (bind _returnvalue (UserInterface|CreateWidget "/Game/UI/WBP_HUD.WBP_HUD_C"))
  (bind _output_get (Variables|Default|SetWBP%20HUD _returnvalue))
  (UserInterface|Viewport|AddtoViewport _output_get 0)
  (CallFunction|GetSimulationManager)
  (Input|AddMappingContext (PlayerController|LocalPlayerSubsystems|GetEnhancedInputLocalPlayerSubsystem) "/Game/Input/InputAction/IMC_SimMappingContext.IMC_SimMappingContext" 0 "(bIgnoreAllPressedKeysUntilRelease=True,bForceImmediately=False,bNotifyUserSettings=False)")
  (UI|SwitchPause))

(fn ConstructionScript)

(fn SwitchPause
  (Variables|Default|GetPauseWidget
    (:then
      (if (Widget|IsVisible (Variables|Default|GetPauseWidget))
        (Widget|SetVisibility (Variables|Default|GetPauseWidget) "Collapsed")
        (Input|SetInputModeGameOnly self false)
        (Variables|Default|SetbShowMouseCursor false)
        (else
          (Widget|SetVisibility (Variables|Default|GetPauseWidget) "Visible")
          (Input|SetInputModeGameandUI self (Variables|Default|GetPauseWidget) "DoNotLock" true false :!label _label)
          (Variables|Default|SetbShowMouseCursor true))))
    (:else
      (UI|CreatePauseWidget)
      (UserInterface|Viewport|AddtoViewport (Variables|Default|GetPauseWidget) 0)
      (goto _label))))

(fn GetSimulationManager
  (bind _returnvalue (Actor|GetActorOfClass "/Game/SimObjects/BP_SimulationManager.BP_SimulationManager_C"))
  (Variables|Default|SetSimulation%20Manager _returnvalue)
  (bind _simulation_manager (Variables|Default|GetSimulation%20Manager)
    (:then
      (EventDispatchers|BindEventtoOnLogAdded _simulation_manager (EventDispatchers|CreateEvent :!event OnEventLogAdded))
      (EventDispatchers|BindEventtoOnScenarioGenerated (Variables|Default|GetSimulation%20Manager) (EventDispatchers|CreateEvent :!event OnScenarioGenerated))
      (EventDispatchers|BindEventtoOnLogAdded (Variables|/Script/SpaceNavigation.SimulationManager|GetRoutePlanner (Variables|Default|GetSimulation%20Manager)) (EventDispatchers|CreateEvent :!event OnPlanLogAdded)))
    (:else)))

(fn OnEventLogAdded
  (params (StringText :type String))
  (bind _simulation_manager (Variables|Default|GetSimulation%20Manager)
    (:then
      (bind _wbp_hud (Variables|Default|GetWBP%20HUD)
        (:then
          (Default|UpdateEventLog _wbp_hud (Variables|/Script/SpaceNavigation.SimulationManager|GetLogs _simulation_manager)))
        (:else)))
    (:else)))

(fn OnPlanLogAdded
  (params (StringText :type String))
  (bind _simulation_manager (Variables|Default|GetSimulation%20Manager)
    (:then
      (bind _wbp_hud (Variables|Default|GetWBP%20HUD)
        (:then
          (Default|UpdatePlanLog _wbp_hud (Variables|/Script/SpaceNavigation.RoutePlanner|GetLogs (Variables|/Script/SpaceNavigation.SimulationManager|GetRoutePlanner _simulation_manager))))
        (:else)))
    (:else)))

(fn CreatePauseWidget
  (bind _returnvalue (UserInterface|CreateWidget "/Game/UI/WBP_Pause.WBP_Pause_C" 0 (Variables|Default|GetSimulation%20Manager)))
  (Variables|Default|SetPauseWidget _returnvalue)
  (CallFunction|PauseBinding)
  (UI|Scenario|SetupScenarioUIConfig)
  (CallFunction|SetupSpacecraftUIConfig)
  (CallFunction|SetupPlanUIConfig))

(fn RestartSimulation
  (bind _simulation_manager (Variables|Default|GetSimulation%20Manager)
    (:then
      (Class|SimulationManager|ResetSimulation _simulation_manager)
      (Class|SimulationManager|StartSimulation (Variables|Default|GetSimulation%20Manager))
      (CallFunction|ResetPawnPosition))
    (:else)))

(fn ExitProgram
  (Game|QuitGame 0 "Quit" false))

(fn OnScenarioConfigChanged
  (params (InNewParams :type Parameters%20Structure%20%28by%20ref%29))
  (bind _simulation_manager (Variables|Default|GetSimulation%20Manager)
    (:then
      (bind _scenariogenerator (Variables|/Script/SpaceNavigation.SimulationManager|GetScenarioGenerator _simulation_manager)
        (:then
          (bind _returnvalue (Class|Importable|ApplyParameters _scenariogenerator InNewParams))
          (if _returnvalue
            (UI|Scenario|SetupScenarioUIConfig)))
        (:else)))
    (:else)))

(fn OnSpacecraftConfigChanged
  (params (InNewParams :type Parameters%20Structure%20%28by%20ref%29))
  (bind _simulation_manager (Variables|Default|GetSimulation%20Manager)
    (:then
      (bind _spacecraft (Variables|/Script/SpaceNavigation.SimulationManager|GetSpacecraft _simulation_manager)
        (:then
          (bind _returnvalue (Class|Importable|ApplyParameters _spacecraft InNewParams))
          (if _returnvalue
            (CallFunction|SetupSpacecraftUIConfig)))
        (:else)))
    (:else)))

(fn OnPlanConfigChanged
  (params (InNewParams :type Parameters%20Structure%20%28by%20ref%29))
  (bind _simulation_manager (Variables|Default|GetSimulation%20Manager)
    (:then
      (bind _routeplanner (Variables|/Script/SpaceNavigation.SimulationManager|GetRoutePlanner _simulation_manager)
        (:then
          (bind _returnvalue (Class|Importable|ApplyParameters _routeplanner InNewParams))
          (if _returnvalue
            (CallFunction|SetupPlanUIConfig)))
        (:else)))
    (:else)))

(fn PauseBinding
  (EventDispatchers|BindEventtoOnContinueClicked (Variables|Default|GetPauseWidget) (EventDispatchers|CreateEvent :!event SwitchPause))
  (EventDispatchers|BindEventtoOnRestartClicked (Variables|Default|GetPauseWidget) (EventDispatchers|CreateEvent :!event RestartSimulation))
  (EventDispatchers|BindEventtoOnExitClicked (Variables|Default|GetPauseWidget) (EventDispatchers|CreateEvent :!event ExitProgram))
  (EventDispatchers|BindEventtoOnApplyScenarioConfig (Variables|Default|GetPauseWidget) (EventDispatchers|CreateEvent :!event OnScenarioConfigChanged))
  (EventDispatchers|BindEventtoOnApplySpacecraftConfig (Variables|Default|GetPauseWidget) (EventDispatchers|CreateEvent :!event OnSpacecraftConfigChanged))
  (EventDispatchers|BindEventtoOnApplyPlan (Variables|Default|GetPauseWidget) (EventDispatchers|CreateEvent :!event OnPlanConfigChanged))
  (EventDispatchers|BindEventtoOnGenerateScenario (Variables|Default|GetPauseWidget) (EventDispatchers|CreateEvent :!event GenerateScenario))
  (EventDispatchers|BindEventtoOnPlanning (Variables|Default|GetPauseWidget) (EventDispatchers|CreateEvent :!event Planning))
  (EventDispatchers|BindEventtoOnSave (Variables|Default|GetPauseWidget) (EventDispatchers|CreateEvent :!event OnSaveScenario))
  (EventDispatchers|BindEventtoOnLoad (Variables|Default|GetPauseWidget) (EventDispatchers|CreateEvent :!event OnLoadScenario)))

(fn GenerateScenario
  (bind _simulation_manager (Variables|Default|GetSimulation%20Manager)
    (:then
      (Class|SimulationManager|GenerateScenario _simulation_manager))
    (:else)))

(fn Planning
  (bind _simulation_manager (Variables|Default|GetSimulation%20Manager)
    (:then
      (Class|SimulationManager|PlanRoute _simulation_manager))
    (:else)))

(fn OnScenarioGenerated
  (CallFunction|ResetPawnPosition))

(fn SetupScenarioUIConfig
  (bind _returnvalue (Class|Importable|ExtractParameters (Variables|/Script/SpaceNavigation.SimulationManager|GetScenarioGenerator (Variables|Default|GetSimulation%20Manager))))
  (Default|SetupScenario (Variables|Default|GetPauseWidget) (Utilities|Struct|BreakParameters _returnvalue)))

(fn SetupSpacecraftUIConfig
  (bind _returnvalue (Class|Importable|ExtractParameters (Variables|/Script/SpaceNavigation.SimulationManager|GetSpacecraft (Variables|Default|GetSimulation%20Manager))))
  (Default|SetupSpacecraft (Variables|Default|GetPauseWidget) (Utilities|Struct|BreakParameters _returnvalue)))

(fn SetupPlanUIConfig
  (bind _returnvalue (Class|Importable|ExtractParameters (Variables|/Script/SpaceNavigation.SimulationManager|GetRoutePlanner (Variables|Default|GetSimulation%20Manager))))
  (Default|SetupPlan (Variables|Default|GetPauseWidget) (Utilities|Struct|BreakParameters _returnvalue)))

(fn ResetPawnPosition
  (LocalVariables|SetNewPawnLocation (+ (Transformation|GetActorLocation (Variables|/Script/SpaceNavigation.SimulationManager|GetSpacecraft (Variables|Default|GetSimulation%20Manager))) (Variables|Default|GetOffsetSpacecraftLookingPosition)))
  (Transformation|SetActorLocation (Pawn|GetControlledPawn) (LocalVariables|GetNewPawnLocation) false false)
  (Pawn|SetControlRotation (Math|Rotator|FindLookatRotation (LocalVariables|GetNewPawnLocation) (Transformation|GetActorLocation (Variables|/Script/SpaceNavigation.SimulationManager|GetSpacecraft (Variables|Default|GetSimulation%20Manager))))))

(fn OnSaveScenario
  (bind _simulation_manager (Variables|Default|GetSimulation%20Manager)
    (:then
      (Class|SimulationManager|ExportConfigtoJsonFile _simulation_manager))
    (:else)))

(fn OnLoadScenario
  (bind _simulation_manager (Variables|Default|GetSimulation%20Manager)
    (:then
      (bind _returnvalue (Class|SimulationManager|ImportConfigfromJsonFile _simulation_manager))
      (if _returnvalue
        (UI|Scenario|SetupScenarioUIConfig)
        (CallFunction|SetupSpacecraftUIConfig)
        (CallFunction|SetupPlanUIConfig)))
    (:else)))