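; Celestial body actor that carries an info widget displaying its body data.
; On BeginPlay it caches the WBP_CelestialInfo instance, enables player input and binds a handler to body initialization.
; SetupInfoWidget copies name, mass and radius from BodyData, and feeds OrbitalRadius into the widget's velocity field.
; The IA_SwitchInfoWidget input action toggles the widget's visibility.
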(event Input|EnhancedActionEvents|EnhancedInputActionIA_SwitchInfoWidget
  (params (ActionValue :type Boolean) (ElapsedSeconds :type Float%20%28double-precision%29) (TriggeredSeconds :type Float%20%28double-precision%29) (InputAction :type Input%20Action%20Object%20Reference :default "/Game/Input/InputAction/IA_SwitchInfoWidget.IA_SwitchInfoWidget"))
  (Rendering|SetVisibility (Variables|Default|GetWidget) (not (Class|WidgetComponent|IsWidgetVisible (Variables|Default|GetWidget))) false))

(event EventBeginPlay
  (bind _aswbp_celestial_info (Utilities|Casting|CastToWBP_CelestialInfo (UserInterface|GetWidget (Variables|Default|GetWidget))))
  (Variables|Default|SetWBP%20Celestial%20Info _aswbp_celestial_info)
  (Input|EnableInput (Game|GetPlayerController 0))
  (EventDispatchers|BindEventtoOnBodyInitialized (EventDispatchers|CreateEvent :!event SetupInfoWidget)))

(event Collision|EventActorBeginOverlap
  (params (OtherActor :type Actor%20Object%20Reference)))

(fn ConstructionScript)

(fn SetupInfoWidget
  (bind _bodydata (Variables|Default|GetBodyData))
  (bind _wbp_celestial_info (Variables|Default|GetWBP%20Celestial%20Info)
    (:then
      (Default|SetMass _wbp_celestial_info (.mass _bodydata))
      (Default|SetRadius (Variables|Default|GetWBP%20Celestial%20Info) (.radius _bodydata))
      (Default|SetVelocity (Variables|Default|GetWBP%20Celestial%20Info) (.orbitalradius _bodydata))
      (Default|SetName (Variables|Default|GetWBP%20Celestial%20Info) (Utilities|Text|ToText(Name) (.bodyname _bodydata))))
    (:else)))