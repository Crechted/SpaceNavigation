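; BP_Spacecraft is a simulated spacecraft actor with an attached widget readout of its mass, fuel and velocity.
; On BeginPlay it caches the widget component's WBP_SpacecraftInfo, then calls UpdateInfo then and every Tick.
; UpdateInfo pushes dry mass, fuel mass, fuel percentage relative to Params, and absolute speed to the widget.
; The construction script writes the craft's Color into the static mesh's custom primitive data.
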(event EventBeginPlay
  (bind _aswbp_spacecraft_info (Utilities|Casting|CastToWBP_SpacecraftInfo (UserInterface|GetWidget (Variables|Default|GetWidget))))
  (Variables|Default|SetWBP%20Spacecraft%20Info _aswbp_spacecraft_info)
  (CallFunction|UpdateInfo))

(event Collision|EventActorBeginOverlap
  (params (OtherActor :type Actor%20Object%20Reference)))

(event EventTick
  (params (DeltaSeconds :type Float%20%28single-precision%29))
  (CallFunction|UpdateInfo))

(fn ConstructionScript
  (bind _color (Variables|Default|GetColor))
  (Rendering|Material|SetCustomPrimitiveDataVector4 (Variables|Default|GetStaticMeshComponent) 0 (Math|Vector4|MakeVector4 (.r _color) (.g _color) (.b _color) (.a _color))))

(fn UpdateInfo
  (bind _params (Variables|Default|GetParams))
  (bind _fuelmasskg (Variables|Default|GetFuelMassKg))
  (bind _wbp_spacecraft_info (Variables|Default|GetWBP%20Spacecraft%20Info)
    (:then
      (Default|SetDryMass _wbp_spacecraft_info (.drymass _params))
      (Default|SetFuelMass (Variables|Default|GetWBP%20Spacecraft%20Info) _fuelmasskg)
      (Default|SetFuelPercent (Variables|Default|GetWBP%20Spacecraft%20Info) (* (/ _fuelmasskg (.fuelmass _params)) 1e+02))
      (Default|SetVelocity (Variables|Default|GetWBP%20Spacecraft%20Info) (Math|Vector|VectorLength (Variables|Default|GetAbsoluteVelocityKmS))))
    (:else)))